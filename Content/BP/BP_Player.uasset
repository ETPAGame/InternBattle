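; BP_Player is the player-controlled character, with movement, look, jump, sprint, crouch and shooting.
; On possession it adds the IMC_Player Enhanced Input mapping context to player controller 0.
; Input actions drive movement along actor axes, scaled yaw and pitch, and walk-speed switching for sprint.
; Shooting spawns a BP_Balle projectile at the OffsetBullet location, with rotation and initial velocity taken from the camera's aim.
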(event `self.ReceivePossessed`
  (params (NewController :type "Controller Object Reference"))
  (bind _returnvalue (pcsubsystem `EnhancedInputLocalPlayerSubsystem` (`GameplayStatics.GetPlayerController` 0)))
  ;[0.9668 0 1] BasicControlPlayer
  (`/Engine/EditorBlueprintResources/StandardMacros.IsValid` _returnvalue
    (:`Is Valid`
      (`EnhancedInputSubsystemInterface.AddMappingContext` _returnvalue "/Game/Input/IMC_Player.IMC_Player" 0 (struct)))))

(event `EnhancedInput|/Game/Input/IA_Look`
  (params (ActionValue :type "Vector2D Structure") (ElapsedSeconds :type "Float (double-precision)") (TriggeredSeconds :type "Float (double-precision)") (InputAction :type "InputAction Object Reference" :default "/Game/Input/IA_Look.IA_Look"))
  (bind _turnrate (`self.TurnRate`))
  ;[0.9668 0 1] BasicControlPlayer
  (:`Triggered`
    (`self.AddControllerYawInput` (* ActionValue_X _turnrate))
    (`self.AddControllerPitchInput` (* ActionValue_Y _turnrate -1.0))))

(event `EnhancedInput|/Game/Input/IA_MoveForward`
  (params (ActionValue :type "Float (double-precision)") (ElapsedSeconds :type "Float (double-precision)") (TriggeredSeconds :type "Float (double-precision)") (InputAction :type "InputAction Object Reference" :default "/Game/Input/IA_MoveForward.IA_MoveForward"))
  ;[0.9668 0 1] BasicControlPlayer
  (:`Triggered`
    (`self.AddMovementInput` (`self.GetActorForwardVector`) (* ActionValue (`self.Speed`)))))

(event `EnhancedInput|/Game/Input/IA_MoveRight`
  (params (ActionValue :type "Float (double-precision)") (ElapsedSeconds :type "Float (double-precision)") (TriggeredSeconds :type "Float (double-precision)") (InputAction :type "InputAction Object Reference" :default "/Game/Input/IA_MoveRight.IA_MoveRight"))
  ;[0.9668 0 1] BasicControlPlayer
  (:`Triggered`
    (`self.AddMovementInput` (`self.GetActorRightVector`) (* (`self.Speed`) ActionValue))))

(event `EnhancedInput|/Game/Input/IA_Jump`
  (params (ActionValue :type Boolean) (ElapsedSeconds :type "Float (double-precision)") (TriggeredSeconds :type "Float (double-precision)") (InputAction :type "InputAction Object Reference" :default "/Game/Input/IA_Jump.IA_Jump"))
  ;[0.9668 0 1] BasicControlPlayer
  (:`Started`
    (`self.Jump`))
  (:`Completed`
    (`self.StopJumping`)))

(event `EnhancedInput|/Game/Input/IA_Sprint`
  (params (ActionValue :type Boolean) (ElapsedSeconds :type "Float (double-precision)") (TriggeredSeconds :type "Float (double-precision)") (InputAction :type "InputAction Object Reference" :default "/Game/Input/IA_Sprint.IA_Sprint"))
  ;[0.9668 0 1] BasicControlPlayer
  (:`Started`
    (set `CharacterMovementComponent.MaxWalkSpeed` (`KismetMathLibrary.SelectFloat` 1200.0 600.0 ActionValue) (`self.CharacterMovement`) :!label _label))
  (:`Completed`
    (goto _label)))

(event `EnhancedInput|/Game/Input/IA_Crouch`
  (params (ActionValue :type Boolean) (ElapsedSeconds :type "Float (double-precision)") (TriggeredSeconds :type "Float (double-precision)") (InputAction :type "InputAction Object Reference" :default "/Game/Input/IA_Crouch.IA_Crouch"))
  ;[0.9668 0 1] BasicControlPlayer
  (:`Started`
    (`self.Crouch`))
  (:`Completed`
    (`self.UnCrouch`)))

(event `EnhancedInput|/Game/Input/IA_Shoot`
  (params (ActionValue :type Boolean) (ElapsedSeconds :type "Float (double-precision)") (TriggeredSeconds :type "Float (double-precision)") (InputAction :type "InputAction Object Reference" :default "/Game/Input/IA_Shoot.IA_Shoot"))
  ;[1 0.02145 0] Shoot
  (:`Started`
    (`|SpawnActorFromClass` "/Game/BP/BP_Balle.BP_Balle_C" (`KismetMathLibrary.MakeTransform` (`SceneComponent.K2_GetComponentLocation` (`self.OffsetBullet`)) (`SceneComponent.K2_GetComponentRotation` (`self.Camera`))) "Undefined" "OverrideRootScale" null (* (`SceneComponent.GetForwardVector` (`self.Camera`)) (`self.InitialBulletSpeed`)) null)))

(fn `UserConstructionScript`)